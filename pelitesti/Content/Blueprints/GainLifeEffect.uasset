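; GainLifeEffect is an effect that alters a PlayerCharacter's LifeForce through its ApplyEffect event, playing a 1-up sound at the world origin.
; It only changes LifeForce when that is already at least 1.0.
; The boost is LifeGain scaled by elapsed game time; sums up to 1.0 are applied and set the effect's Speed very high, while larger sums clamp LifeForce to 1.0.
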(event EventBeginPlay)

(event Collision|EventActorBeginOverlap
  (params (OtherActor :type Actor%20Object%20Reference)))

(event EventTick
  (params (DeltaSeconds :type Float%20%28single-precision%29)))

(event EventApplyEffect
  (params (PlayerCharacter :type BB%20My%20Character%20Object%20Reference))
  ;[1 1 1] Check hp
  (Audio|PlaySoundatLocation "/Game/Sounds/smw_1-up.smw_1-up" "0, 0, 0" "0, 0, 0" 1.0 1.0 0.0 0 0 0)
  (if (>= (Variables|/Game/Blueprints/BB_MyCharacter.BB_MyCharacter_C|GetlifeForce PlayerCharacter) 1.0)
    ;[1 1 1] Check if hp full or not and increase it from boosted value
    (if (<= (+ (Variables|/Game/Blueprints/BB_MyCharacter.BB_MyCharacter_C|GetlifeForce PlayerCharacter) (* (/ (Utilities|Time|GetGameTimeinSeconds) 5.0) (Variables|Default|GetlifeGain))) 1.0)
      (Variables|/Game/Blueprints/BB_MyCharacter.BB_MyCharacter_C|SetlifeForce PlayerCharacter (+ (Variables|/Game/Blueprints/BB_MyCharacter.BB_MyCharacter_C|GetlifeForce PlayerCharacter) (* (/ (Utilities|Time|GetGameTimeinSeconds) 5.0) (Variables|Default|GetlifeGain))))
      (Variables|Default|SetSpeed 1e+04)
      (else
        (Variables|/Game/Blueprints/BB_MyCharacter.BB_MyCharacter_C|SetlifeForce PlayerCharacter 1.0)))))

(fn ConstructionScript
  (|CallParentFunction))