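; GroundEnemy is a hazard actor that drains the player character's LifeForce on contact.
; On overlap it identifies BB_MyCharacter by display name, casts to it and plays a laser sound at the world origin.
; It then subtracts LifeDrain scaled by elapsed game time, so hits grow stronger over time, and floors LifeForce at zero.
; The ApplyEffect function and construction script are empty.
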(event EventBeginPlay)

(event EventTick
  (params (DeltaSeconds :type Float%20%28single-precision%29)))

(event Collision|EventActorBeginOverlap
  (params (OtherActor :type Actor%20Object%20Reference))
  ;[1 1 1] Checks overlapping with the character
  (if (Utilities|Enum|Equal(Enum) (Utilities|GetDisplayName OtherActor) "BB_MyCharacter")
    (bind _asbb_my_character (Utilities|Casting|CastToBB_MyCharacter OtherActor))
    (Audio|SpawnSoundatLocation "/Game/Sounds/space_laser_shot.space_laser_shot" "0, 0, 0" "0, 0, 0" 1.0 1.0 0.0 0 0)
    ;[1 1 1] Check if hp full or not and increase it from boosted value
    (if (> (- (Variables|/Game/Blueprints/BB_MyCharacter.BB_MyCharacter_C|GetlifeForce _asbb_my_character) (* (/ (Utilities|Time|GetGameTimeinSeconds) 5.0) (Variables|Default|GetlifeDrain))) 0.0)
      (Variables|/Game/Blueprints/BB_MyCharacter.BB_MyCharacter_C|SetlifeForce _asbb_my_character (- (Variables|/Game/Blueprints/BB_MyCharacter.BB_MyCharacter_C|GetlifeForce _asbb_my_character) (* (/ (Utilities|Time|GetGameTimeinSeconds) 5.0) (Variables|Default|GetlifeDrain))))
      (else
        (Variables|/Game/Blueprints/BB_MyCharacter.BB_MyCharacter_C|SetlifeForce _asbb_my_character 0.0)))))

(fn ConstructionScript)

(fn ApplyEffect
  (params (PlayerCharacter :type BB%20My%20Character%20Object%20Reference)))