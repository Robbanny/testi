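; GainSpeedEffect is an effect Blueprint, named for granting speed, that exposes an ApplyEffect event taking a player character.
; ApplyEffect checks whether the character's forward acceleration is below a threshold and, if so, sets a Speed variable to a fixed value.
; An addition on the character's forward acceleration is left unconnected, so the graph never changes that acceleration.
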(event EventBeginPlay
  (|CallParentFunction) ; This node is disabled and will not be called.\nDrag off pins to build functionality.
)

(event Collision|EventActorBeginOverlap
  (params (OtherActor :type Actor%20Object%20Reference))
  (|CallParentFunction OtherActor) ; This node is disabled and will not be called.\nDrag off pins to build functionality.
)

(event EventTick
  (params (DeltaSeconds :type Float%20%28single-precision%29))
  (|CallParentFunction DeltaSeconds) ; This node is disabled and will not be called.\nDrag off pins to build functionality.
)

(event EventApplyEffect
  (params (PlayerCharacter :type BB%20My%20Character%20Object%20Reference))
  (if (< (Variables|/Game/Blueprints/BB_MyCharacter.BB_MyCharacter_C|GetForwardAcceleration PlayerCharacter) 6e+01)
    (Variables|Default|SetSpeed 5e+02)))

(fn ConstructionScript
  (|CallParentFunction))