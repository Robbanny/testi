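; AvoidablesPool is an object pool for side-scrolling Collectible actors that travel leftward across the screen.
; CreateCollectible spawns a random class at the start X and random height until the cap is reached, with a game-time-dependent random speed.
; UpdateCollectible moves each pooled actor per call, recycling those past the left bound to the start with new height and speed instead of respawning.
; Its own event graph is empty, so neither function is triggered here.
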(event EventBeginPlay)

(event Collision|EventActorBeginOverlap
  (params (OtherActor :type Actor%20Object%20Reference)))

(event EventTick
  (params (DeltaSeconds :type Float%20%28single-precision%29)))

(fn ConstructionScript)

(fn CreateCollectible
  (bind _collectibles (Variables|Default|Getcollectibles))
  ;[1 1 1] Only create collectible if max amount has not been reached
  (if (< (Variables|Default|GetnumberOfCollectibles) (Variables|Default|GetmaxNumberOfCollectible))
    ;[1 1 1] Create collectible into the scene and adjust position and speed
    (bind _returnvalue (Game|SpawnActorfromClass (Utilities|Array|Get(acopy) _collectibles (Math|Random|RandomIntegerinRange 0 (Utilities|Array|LastIndex _collectibles))) (Math|Transform|MakeTransform (Math|Vector|MakeVector (Variables|Default|GetcollectibleStartX) 0.0 (Math|Random|RandomFloatinRange 2e+02 5e+02))) "Undefined" 0 0))
    (bind _ascollectible (Utilities|Casting|CastToCollectible _returnvalue))
    (Variables|/Game/Blueprints/Collectible.Collectible_C|SetSpeed _ascollectible (Math|Random|RandomFloatinRange (/ (Variables|/Game/Blueprints/Collectible.Collectible_C|GetSpeed _ascollectible) (/ (Utilities|Time|GetGameTimeinSeconds) 1e+01)) (Variables|/Game/Blueprints/Collectible.Collectible_C|GetSpeed _ascollectible)))
    ;[1 1 1] add created collectible to pool and increment counter
    (Utilities|Array|Insert (Variables|Default|GetThePool) _ascollectible (Variables|Default|GetnumberOfCollectibles))
    (Math|Integer|IncrementInt (Variables|Default|GetnumberOfCollectibles))))

(fn UpdateCollectible
  ;[1 1 1] update each collectible in the pool
  (for (_array_element _array_index) (Variables|Default|GetThePool)
    ;[1 1 1] Check if object is far enough on the left side of the screen to be able to appear again
    (LocalVariables|SetarrayElement _array_element)
    (LocalVariables|SetarrayIndex _array_index)
    (if (< (.X (Math|Vector|BreakVector (Transformation|GetWorldLocation (Variables|/Script/Engine.Actor|GetRootComponent _array_element)))) (- 0.0 (Variables|Default|GetcollectibleStartX)))
      ;[1 1 1] "create" collectible into the scene and adjust position and speed
      (Transformation|SetWorldLocation (Variables|/Script/Engine.Actor|GetRootComponent (LocalVariables|GetarrayElement)) (Math|Vector|MakeVector (Variables|Default|GetcollectibleStartX) 0.0 (Math|Random|RandomFloatinRange -5e+01 5e+02)) false false)
      (bind _ascollectible (Utilities|Casting|CastToCollectible (LocalVariables|GetarrayElement)))
      (Variables|/Game/Blueprints/Collectible.Collectible_C|SetSpeed _ascollectible (Math|Random|RandomFloatinRange 15.0 25.0))
      (else
        ;[1 1 1] If not too far on the left, move object
        (bind _ascollectible_2 (Utilities|Casting|CastToCollectible _array_element))
        (Transformation|AddWorldOffset (Variables|/Script/Engine.Actor|GetRootComponent _array_element) (Math|Vector|MakeVector (- 0.0 (Variables|/Game/Blueprints/Collectible.Collectible_C|GetSpeed _ascollectible_2)) 0.0 0.0) false false)))))