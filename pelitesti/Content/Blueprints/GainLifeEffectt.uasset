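; GainLifeEffectt is an effect Blueprint that restores LifeForce on a BB_MyCharacter when ApplyEffect fires.
; It acts only while LifeForce is below 1.0 and caps the result at that maximum.
; The heal amount is the Effect value scaled by elapsed game time, so the boost grows stronger the longer the game runs.
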(event EventBeginPlay)

(event Collision|EventActorBeginOverlap
  (params (OtherActor :type Actor%20Object%20Reference)))

(event EventTick
  (params (DeltaSeconds :type Float%20%28single-precision%29)))

(event EventApplyEffect
  (params (PlayerCharacter :type BB%20My%20Character%20Object%20Reference))
  (bind _asbb_my_character (Utilities|Casting|CastToBB_MyCharacter))
  ;[1 1 1] Check hp
  (if (< (Variables|/Game/Blueprints/BB_MyCharacter.BB_MyCharacter_C|GetlifeForce _asbb_my_character) 1.0)
    ;[1 1 1] Check if hp full or not and increase it from boosted value
    (if (<= (+ (Variables|/Game/Blueprints/BB_MyCharacter.BB_MyCharacter_C|GetlifeForce _asbb_my_character) (* (/ (Utilities|Time|GetGameTimeinSeconds) 5.0) (Variables|Default|GetEffect))) 1.0)
      (Variables|/Game/Blueprints/BB_MyCharacter.BB_MyCharacter_C|SetlifeForce _asbb_my_character (+ (Variables|/Game/Blueprints/BB_MyCharacter.BB_MyCharacter_C|GetlifeForce _asbb_my_character) (* (/ (Utilities|Time|GetGameTimeinSeconds) 5.0) (Variables|Default|GetEffect))))
      (else
        (Variables|/Game/Blueprints/BB_MyCharacter.BB_MyCharacter_C|SetlifeForce _asbb_my_character 1.0)))))

(fn ConstructionScript
  (|CallParentFunction))