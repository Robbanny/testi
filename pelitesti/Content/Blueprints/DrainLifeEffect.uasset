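; DrainLifeEffect is an effect Blueprint that lowers the player character's LifeForce when ApplyEffect is called.
; The drain is LifeDrain scaled by total game time rather than delta time, so each call removes more as the game runs.
; The result is capped at 1.0 with no lower clamp.
; The HP check branch is hard-wired to true, and BeginPlay, overlap and Tick are disabled stubs.
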(event EventBeginPlay
  (|CallParentFunction) ; This node is disabled and will not be called.\nDrag off pins to build functionality.
)

(event Collision|EventActorBeginOverlap
  (params (OtherActor :type Actor%20Object%20Reference))
  (|CallParentFunction OtherActor) ; This node is disabled and will not be called.\nDrag off pins to build functionality.
)

(event EventTick
  (params (DeltaSeconds :type Float%20%28single-precision%29))
  (|CallParentFunction DeltaSeconds) ; This node is disabled and will not be called.\nDrag off pins to build functionality.
)

(event EventApplyEffect
  (params (PlayerCharacter :type BB%20My%20Character%20Object%20Reference))
  ;[1 1 1] Check hp
  (if true
    ;[1 1 1] Check if hp full or not and increase it from boosted value
    (if (<= (- (Variables|/Game/Blueprints/BB_MyCharacter.BB_MyCharacter_C|GetlifeForce PlayerCharacter) (* (/ (Utilities|Time|GetGameTimeinSeconds) 5.0) (Variables|Default|GetlifeDrain))) 1.0)
      (Variables|/Game/Blueprints/BB_MyCharacter.BB_MyCharacter_C|SetlifeForce PlayerCharacter (- (Variables|/Game/Blueprints/BB_MyCharacter.BB_MyCharacter_C|GetlifeForce PlayerCharacter) (* (/ (Utilities|Time|GetGameTimeinSeconds) 5.0) (Variables|Default|GetlifeDrain))))
      (else
        (Variables|/Game/Blueprints/BB_MyCharacter.BB_MyCharacter_C|SetlifeForce PlayerCharacter 1.0)))))

(fn ConstructionScript
  (|CallParentFunction))