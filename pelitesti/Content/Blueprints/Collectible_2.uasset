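; Collectible_2 is a healing collectible that restores the player character's LifeForce when its Box component is overlapped.
; The overlap event matches the other actor by display name "BB_MyCharacter" before casting, then heals only if LifeForce is below full.
; The heal scales the Effect variable by elapsed game time, so it grows as play continues, and clamps LifeForce at 1.0.
; The graph does not destroy or disable the collectible afterwards.
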(event OnComponentBeginOverlap(Box)
  (params (OverlappedComponent :type Primitive%20Component%20Object%20Reference) (OtherActor :type Actor%20Object%20Reference) (OtherComp :type Primitive%20Component%20Object%20Reference) (OtherBodyIndex :type Integer) (bFromSweep :type Boolean) (SweepResult :type Hit%20Result%20Structure%20%28by%20ref%29))
  ;[1 1 1] Checks overlapping with the character
  (if (Utilities|Enum|Equal(Enum) (Utilities|GetDisplayName OtherActor) "BB_MyCharacter")
    (bind _asbb_my_character (Utilities|Casting|CastToBB_MyCharacter OtherActor))
    ;[1 1 1] Check hp
    (if (< (Variables|/Game/Blueprints/BB_MyCharacter.BB_MyCharacter_C|GetlifeForce _asbb_my_character) 1.0)
      ;[1 1 1] Check if hp full or not and increase it from boosted value
      (if (<= (+ (Variables|/Game/Blueprints/BB_MyCharacter.BB_MyCharacter_C|GetlifeForce _asbb_my_character) (* (/ (Utilities|Time|GetGameTimeinSeconds) 5.0) (Variables|Default|GetEffect))) 1.0)
        (Variables|/Game/Blueprints/BB_MyCharacter.BB_MyCharacter_C|SetlifeForce _asbb_my_character (+ (Variables|/Game/Blueprints/BB_MyCharacter.BB_MyCharacter_C|GetlifeForce _asbb_my_character) (* (/ (Utilities|Time|GetGameTimeinSeconds) 5.0) (Variables|Default|GetEffect))))
        (else
          (Variables|/Game/Blueprints/BB_MyCharacter.BB_MyCharacter_C|SetlifeForce _asbb_my_character 1.0))))))

(event EventBeginPlay)

(event Collision|EventActorBeginOverlap
  (params (OtherActor :type Actor%20Object%20Reference)))

(event EventTick
  (params (DeltaSeconds :type Float%20%28single-precision%29)))

(fn ConstructionScript)